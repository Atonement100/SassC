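; Lobby GameState that stores the host's name and tallies players' map votes.
; On BeginPlay it scans PlayerArray and records the name of a player state with authority as host.
; Vote requests reject names already in the voted list and print the result.
; The tally looks unfinished: it only increments Orbit, resetting Random, when the map choice is an empty string.
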(event Custom|playerWantsToVote
  (params (PlayerName :type String) (MapChoice :type String))
  (if (>= (Utilities|Array|FindItem (Variables|Default|GetaPlayersHaveVotedArray) PlayerName) 0)
    (Development|PrintString (Utilities|String|Append PlayerName "has already voted."))
    (else
      (bind (_array_element _array_index) (Utilities|Array|ForEachLoopwithBreak (Variables|Default|GetaMapVoteArray) :!label _label)
        (:LoopBody
          (if (Utilities|Enum|Equal(Enum) "" MapChoice)
            (Utilities|Array|SetArrayElem (Variables|Default|GetaMapVoteArray) _array_index (Utilities|Struct|MakemapVoteStruct (+ (.orbit (Utilities|Struct|BreakmapVoteStruct _array_element)) 1)))
            (Utilities|Array|Add (Variables|Default|GetaPlayersHaveVotedArray) PlayerName)
            (goto _label Break)))
        (:Completed
          (Development|PrintString (Utilities|String|Append (Utilities|String|Append PlayerName " voted for ") MapChoice)))))))

(event EventBeginPlay
  (CallFunction|SetHostName))

(event EventTick
  (params (DeltaSeconds :type Float%20%28single-precision%29)))

(fn ConstructionScript)

(fn SetHostName
  (bind _array_element (Utilities|Array|ForEachLoopwithBreak (Variables|Default|GetPlayerArray) :!label _label)
    (:LoopBody
      (if (Ability|HasAuthority _array_element)
        (Utilities|FlowControl|Sequence
          (:then_0
            (goto _label Break))
          (:then_1
            (Variables|Default|Setnameofhost (PlayerState|GetPlayerName _array_element))))))
    (:Completed
      _))
  (return))