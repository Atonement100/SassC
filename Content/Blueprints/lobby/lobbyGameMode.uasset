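; Lobby game mode that assigns player IDs and holds an unfinished map-vote system.
; On PostLogin, it sets each player's LobbyPlayerID to one above that of the last PlayerArray entry.
; The disconnected vote sequence resets game-state arrays, opens a timed window, then tallies Orbit votes through helper functions and prints the result.
; StartMapVote is empty, and random-map selection remains a placeholder.
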(event Custom|StartMapVote)

(event EventBeginPlay)

(event EventTick
  (params (DeltaSeconds :type Float%20%28single-precision%29)))

(event EventPostLogin
  (params (NewPlayer :type Player%20Controller%20Object%20Reference))
  (bind _returnvalue (Game|GetGameState))
  (bind _playerstate (Variables|/Script/Engine.Controller|GetPlayerState NewPlayer))
  (Utilities|IsValid _playerstate
    (:Is%20Valid
      (bind _assass_lobby_player_state (Utilities|Casting|CastTosassLobbyPlayerState _playerstate))
      (Utilities|IsValid _returnvalue
        (:Is%20Valid
          (bind _assass_lobby_game_state (Utilities|Casting|CastTosassLobbyGameState _returnvalue))
          (if (> (Utilities|Array|Length (Variables|/Script/Engine.GameState|GetPlayerArray _assass_lobby_game_state)) 0)
            (bind _assass_lobby_player_state_2 (Utilities|Casting|CastTosassLobbyPlayerState (Utilities|Array|Get(acopy) (Variables|/Script/Engine.GameState|GetPlayerArray _assass_lobby_game_state) (Utilities|Array|LastIndex (Variables|/Script/Engine.GameState|GetPlayerArray _assass_lobby_game_state)))))
            (Variables|/Game/Blueprints/lobby/sassLobbyPlayerState.sassLobbyPlayerState_C|SetlobbyPlayerID _assass_lobby_player_state (+ (Variables|/Game/Blueprints/lobby/sassLobbyPlayerState.sassLobbyPlayerState_C|GetlobbyPlayerID _assass_lobby_player_state_2) 1))
            (else
              (Variables|/Game/Blueprints/lobby/sassLobbyPlayerState.sassLobbyPlayerState_C|SetlobbyPlayerID _assass_lobby_player_state 0))))))))

(fn ConstructionScript)

(fn ResetVoteArrays
  (params (self2 :type Sass%20Lobby%20Game%20State%20Object%20Reference))
  (bind _amapvotearray (Variables|/Game/Blueprints/lobby/sassLobbyGameState.sassLobbyGameState_C|GetaMapVoteArray self2))
  (Utilities|Array|Clear (Variables|/Game/Blueprints/lobby/sassLobbyGameState.sassLobbyGameState_C|GetaPlayersHaveVotedArray self2))
  (Utilities|Array|Clear (Variables|/Game/Blueprints/lobby/sassLobbyGameState.sassLobbyGameState_C|GetaWinningMapsArray self2))
  (for (_array_element _array_index) _amapvotearray
    (Utilities|Array|SetArrayElem _amapvotearray _array_index (Utilities|Struct|MakemapVoteStruct))))