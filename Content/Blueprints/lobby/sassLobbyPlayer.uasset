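; Player character for the lobby, handling movement, camera look, the local HUD, pause menu and voting menus.
; Sprint and crouch pass their state to OnServer events that set walk speed; crouch also changes eye height but gives a higher speed than sprint.
; Q toggles a map-vote or general vote widget based on the lobby GameState, Escape toggles pause, and F10 quits.
; An object line trace is present but never runs.
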(event Custom|playerCrouchOnServer
  (params (isCrouched :type Boolean))
  (bind _charactermovement (Variables|Character|GetCharacterMovement))
  ;[1 1 1] Crouching
  (if isCrouched
    (Variables|/Script/Engine.CharacterMovementComponent|SetMaxWalkSpeed _charactermovement 2e+03)
    (else
      (Variables|/Script/Engine.CharacterMovementComponent|SetMaxWalkSpeed _charactermovement 4e+02))))

(event Custom|playerRunOnServer
  (params (isRunning :type Boolean))
  (bind _charactermovement (Variables|Character|GetCharacterMovement))
  ;[1 1 1] Sprinting
  (if isRunning
    (Variables|/Script/Engine.CharacterMovementComponent|SetMaxWalkSpeed _charactermovement 8e+02)
    (else
      (Variables|/Script/Engine.CharacterMovementComponent|SetMaxWalkSpeed _charactermovement 4e+02))))

(event EventBeginPlay
  ;[1 1 1] Player spawning, hud creation
  (Utilities|FlowControl|Delay 0.2)
  (if (not (Networking|IsDedicatedServer))
    (if (Pawn|IsLocalController (Game|GetPlayerController 0))
      (if (not (Variables|Default|GetHUDCreated))
        (bind _returnvalue (UserInterface|CreateWidget "/Game/Blueprints/lobby/lobbyHUD.lobbyHUD_C"))
        (Variables|Default|SetlobbyHudWidget _returnvalue)
        (UserInterface|Viewport|AddtoViewport _returnvalue 0)
        (Variables|Default|SetHUDCreated true)))))

(event Collision|EventActorBeginOverlap
  (params (OtherActor :type Actor%20Object%20Reference)))

(event EventTick
  (params (DeltaSeconds :type Float%20%28single-precision%29)))

(event Input|ActionEvents|InputActionJump
  (params (Key :type Key%20Structure :default "None"))
  (:Pressed
    (Character|Jump)))

(event Input|ActionEvents|InputActionCrouch
  (params (Key :type Key%20Structure :default "None"))
  ;[1 1 1] Crouching
  (:Pressed
    (Variables|Default|SetCrouchPressed true)
    (Variables|Default|SetBaseEyeHeight 4e+01)
    (CallFunction|PlayerCrouchonServer (Variables|Default|GetCrouchPressed) :!label _label))
  (:Released
    (Variables|Default|SetCrouchPressed false)
    (Variables|Default|SetBaseEyeHeight 8e+01)
    (goto _label)))

(event Input|ActionEvents|InputActionSprint
  (params (Key :type Key%20Structure :default "None"))
  ;[1 1 1] Sprinting
  (:Pressed
    (Variables|Default|SetSprintPressed true)
    (Variables|Default|SetCrouchPressed false)
    (CallFunction|PlayerRunonServer (Variables|Default|GetSprintPressed) :!label _label))
  (:Released
    (Variables|Default|SetSprintPressed false)
    (goto _label)))

(event Input|AxisEvents|InputAxisYawCamera
  (params (AxisValue :type Float%20%28single-precision%29))
  ;[1 1 1] Turning & Movement
  (Pawn|Input|AddControllerYawInput (* AxisValue (Variables|Default|GetmenuRotationModifier))))

(event Input|AxisEvents|InputAxisPitchCamera
  (params (AxisValue :type Float%20%28single-precision%29))
  (bind _menurotationmodifier (Variables|Default|GetmenuRotationModifier))
  (bind _returnvalue (* AxisValue _menurotationmodifier))
  ;[1 1 1] Turning & Movement
  (if (Variables|Default|GetInvertLookUp)
    (Pawn|Input|AddControllerPitchInput (* -1.0 _returnvalue))
    (else
      (Pawn|Input|AddControllerPitchInput _returnvalue))))

(event Input|AxisEvents|InputAxisMoveForward
  (params (AxisValue :type Float%20%28single-precision%29))
  ;[1 1 1] Turning & Movement
  (Pawn|Input|AddMovementInput (Math|Vector|GetForwardVector (Math|Rotator|MakeRotator 0.0 0.0 (.Yaw (Math|Rotator|BreakRotator (Pawn|GetControlRotation :!class /Script/Engine.Pawn))))) AxisValue false))

(event Input|AxisEvents|InputAxisMoveRight
  (params (AxisValue :type Float%20%28single-precision%29))
  ;[1 1 1] Turning & Movement
  (Pawn|Input|AddMovementInput (Math|Vector|GetRightVector (Math|Rotator|MakeRotator 0.0 0.0 (.Yaw (Math|Rotator|BreakRotator (Pawn|GetControlRotation :!class /Script/Engine.Pawn))))) AxisValue false))

(event Input|KeyboardEvents|F10
  (params (Key :type Key%20Structure :default "None"))
  (:Pressed
    (Game|QuitGame 0 "Quit" false)))

(event Input|KeyboardEvents|Escape
  (params (Key :type Key%20Structure :default "None"))
  (bind _returnvalue (Game|GetPlayerController 0))
  ;[1 1 1] Pausing
  (:Pressed
    (if (not (Variables|Default|GetbIsPaused))
      (bind _returnvalue_2 (UserInterface|CreateWidget "/Game/Blueprints/common/lobbyPauseMenu.lobbyPauseMenu_C" _returnvalue))
      (Variables|Default|SetpauseMenuWidget _returnvalue_2)
      (UserInterface|Viewport|AddtoViewport _returnvalue_2 0)
      (Input|SetInputModeGameandUI _returnvalue 0 "LockAlways" true false)
      (Variables|/Script/Engine.PlayerController|SetbShowMouseCursor _returnvalue true)
      (Variables|Default|SetbIsPaused true)
      (Input|SetIgnoreMoveInput (Game|GetPlayerController 0) true)
      (else
        (CallFunction|Unpause _returnvalue_2 _returnvalue)))))

(event Input|KeyboardEvents|Q
  (params (Key :type Key%20Structure :default "None"))
  (bind _returnvalue (Game|GetPlayerController 0))
  (bind _returnvalue_2 (Game|GetPlayerController 0))
  (bind _returnvalue_3 (Game|GetGameState))
  ;[1 1 1] Map Vote Handling
  (:Pressed
    (if (Variables|Default|GetbIsMapVoteHUDOpen)
      (Widget|RemovefromParent (Variables|Default|GetActiveLobbyVoteWidget))
      (Input|SetInputModeGameOnly _returnvalue_2 false)
      (Variables|/Script/Engine.PlayerController|SetbShowMouseCursor _returnvalue_2 false)
      (Variables|Default|SetbIsMapVoteHUDOpen false)
      (else
        (Utilities|IsValid _returnvalue_3
          (:Is%20Valid
            (bind _assass_lobby_game_state (Utilities|Casting|CastTosassLobbyGameState _returnvalue_3))
            (if (Variables|/Game/Blueprints/lobby/sassLobbyGameState.sassLobbyGameState_C|GetisMapVoteActive _assass_lobby_game_state)
              (bind _returnvalue_4 (UserInterface|CreateWidget "/Game/Blueprints/lobby/lobbyMapVoteMenuHUD.lobbyMapVoteMenuHUD_C" _returnvalue))
              (Variables|Default|SetActiveLobbyVoteWidget _returnvalue_4)
              (UserInterface|Viewport|AddtoViewport _returnvalue_4 1)
              (else
                (bind _returnvalue_5 (UserInterface|CreateWidget "/Game/Blueprints/lobby/lobbyVoteMenuHUD.lobbyVoteMenuHUD_C" _returnvalue))
                (Variables|Default|SetActiveLobbyVoteWidget _returnvalue_5)
                (UserInterface|Viewport|AddtoViewport _returnvalue_5 1)))
            (Input|SetInputModeGameandUI _returnvalue 0 "LockAlways" false false)
            (Variables|/Script/Engine.PlayerController|SetbShowMouseCursor _returnvalue true)
            (Variables|Default|SetbIsMapVoteHUDOpen true)))))))

(fn ConstructionScript)

(fn Unpause
  (params (WidgetToRemove :type Widget%20Object%20Reference) (PlayerController :type Player%20Controller%20Object%20Reference))
  (Widget|RemovefromParent WidgetToRemove)
  (Input|SetInputModeGameOnly PlayerController false)
  (Variables|/Script/Engine.PlayerController|SetbShowMouseCursor PlayerController false)
  (Variables|Default|SetbIsPaused false)
  (Input|SetIgnoreMoveInput PlayerController false))