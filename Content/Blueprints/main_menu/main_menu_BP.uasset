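; Main menu controller that shows the menu widget on BeginPlay, clears leftover lobby and game HUDs, and manages multiplayer sessions.
; openLobby creates a LAN or online session and opens the lobby level as a listen server.
; findLobbies searches for sessions and fills the join widget's scrollbox with one entry per result, toggling searching, empty and refresh states.
; Other events join a selected result, clear old entries and collapse the join widget.
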(event Custom|findLobbies
  (Utilities|IsValid (Variables|Default|GetmainMenuJoinWidget)
    (:Is%20Valid
      (Widget|SetVisibility (Variables|Default|GetmainMenuJoinWidget) "Visible"))
    (:Is%20Not%20Valid
      (bind _returnvalue (UserInterface|CreateWidget "/Game/Blueprints/main_menu/main_menu_join.main_menu_join_C" (Game|GetPlayerController 0)))
      (Variables|Default|SetmainMenuJoinWidget _returnvalue)
      (UserInterface|Viewport|AddtoViewport _returnvalue 2)))
  (Default|NoServersFoundCollapsed (Variables|Default|GetmainMenuJoinWidget))
  (Default|SearchingVisible (Variables|Default|GetmainMenuJoinWidget))
  (Default|RefreshCollapsed (Variables|Default|GetmainMenuJoinWidget))
  (bind _results (|FindSessions (Game|GetPlayerController 0) 100 (Variables|Default|GetuseLAN))
    (:OnSuccess
      (Variables|Default|SetfoundSessions _results)
      (if (== (Utilities|Array|Length _results) 0)
        (Default|SearchingCollapsed (Variables|Default|GetmainMenuJoinWidget) :!label _label)
        (Default|NoServersFoundVisible (Variables|Default|GetmainMenuJoinWidget))
        (Default|RefreshVisible (Variables|Default|GetmainMenuJoinWidget))
        (else
          (Default|SearchingCollapsed (Variables|Default|GetmainMenuJoinWidget))
          (for _array_element (Variables|Default|GetfoundSessions)
            (bind _returnvalue_2 (UserInterface|CreateWidget "/Game/Blueprints/main_menu/main_menu_join_entry.main_menu_join_entry_C" (Game|GetPlayerController 0)))
            (Utilities|Array|Add (Variables|Default|GetfoundSessionsWidgets) _returnvalue_2)
            (bind _output_get (Variables|Default|SetmainMenuJoinEntryWidget _returnvalue_2))
            (Default|SetName _output_get (Utilities|CreateServerString _array_element))
            (Default|SetSearchResult _output_get _array_element)
            (Widget|Panel|AddChild (Variables|/Game/Blueprints/main_menu/main_menu_join.main_menu_join_C|GetServerScrollbox (Variables|Default|GetmainMenuJoinWidget)) _output_get))
          (Default|RefreshVisible (Variables|Default|GetmainMenuJoinWidget)))))
    (:OnFailure
      (goto _label))))

(event Custom|destroyLobbiesWidget
  (Widget|SetVisibility (Variables|Default|GetmainMenuJoinWidget) "Collapsed"))

(event Custom|openLobby
  (params (useLan :type Boolean))
  (bind _returnvalue (Game|GetPlayerController 0))
  (bind _output_get (Variables|Default|SetuseLAN useLan))
  (|Session (Game|GetPlayerController 0) 8 _output_get
    (:OnSuccess
      (Development|PrintString "session created")
      (Widget|RemovefromParent (Variables|Default|GetmainMenuWidget))
      (Game|OpenLevel(byName) "lobby" true "listen")
      (Input|SetInputModeGameOnly _returnvalue false)
      (Variables|/Script/Engine.PlayerController|SetbShowMouseCursor _returnvalue false))
    (:OnFailure
      (Development|PrintString "session not created"))))

(event Custom|joinSelectedLobby
  (params (Result :type Blueprint%20Session%20Result%20Structure))
  (|JoinSession (Game|GetPlayerController 0) Result
    (:OnSuccess
      (Development|PrintString "Session successfully joined!")
      (Widget|RemovefromParent (Variables|Default|GetmainMenuWidget))
      (Widget|RemovefromParent (Variables|Default|GetmainMenuJoinWidget)))
    (:OnFailure
      (Development|PrintString "ERR: COULD NOT JOIN SESSION"))))

(event Custom|deleteOldLobbies
  (bind _foundsessionswidgets (Variables|Default|GetfoundSessionsWidgets))
  (for _array_element _foundsessionswidgets
    (Class|PanelWidget|RemoveChild (Variables|/Game/Blueprints/main_menu/main_menu_join.main_menu_join_C|GetServerScrollbox (Variables|Default|GetmainMenuJoinWidget)) _array_element))
  (Utilities|Array|Clear _foundsessionswidgets))

(event EventBeginPlay
  (bind _returnvalue (UserInterface|CreateWidget "/Game/Blueprints/main_menu/main_menu.main_menu_C"))
  (Variables|Default|SetmainMenuWidget _returnvalue)
  (UserInterface|Viewport|AddtoViewport _returnvalue 0)
  (Variables|/Script/Engine.PlayerController|SetbShowMouseCursor (Game|GetPlayerController 0) true)
  (Utilities|CleanAllMenus))

(event EventTick
  (params (DeltaSeconds :type Float%20%28single-precision%29)))

(fn ConstructionScript)