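; BP_NodeContainer is an actor that holds the BP_GraphNode actors of the territory system and offers bulk operations on them.
; RemoveAllNodes destroys every actor in its Nodes array, first filling it from all BP_GraphNode actors in the world if it is empty, and prints the remaining count.
; ToggleNodeVisibility flips the root component's visibility and propagates it to child components.
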(event EventBeginPlay)

(event Collision|EventActorBeginOverlap
  (params (OtherActor :type Actor%20Object%20Reference)))

(event EventTick
  (params (DeltaSeconds :type Float%20%28single-precision%29)))

(fn ConstructionScript)

(fn RemoveAllNodes
  (if (Utilities|Array|IsNotEmpty (Variables|Default|GetNodes))
    _
    (else
      (bind _outactors (Actor|GetAllActorsOfClass "/Game/Blueprints/sassilization/Territory/BP_GraphNode.BP_GraphNode_C"))
      (Variables|Default|SetNodes _outactors)))
  (while (Utilities|Array|IsNotEmpty (Variables|Default|GetNodes))
    (Actor|DestroyActor (Utilities|Array|Get(acopy) (Variables|Default|GetNodes)))
    (Utilities|Array|RemoveIndex (Variables|Default|GetNodes))
    (Development|PrintString (Utilities|String|BuildString(Integer) "" "destroyed another child, with x remaining: " (Utilities|Array|Length (Variables|Default|GetNodes))) false))
  (Development|PrintString (Utilities|String|ToString(Integer) (Utilities|Array|Length (Variables|Default|GetNodes)))))

(fn ToggleNodeVisibility
  (Rendering|ToggleVisibility (Variables|Transformation|GetRootComponent) true))