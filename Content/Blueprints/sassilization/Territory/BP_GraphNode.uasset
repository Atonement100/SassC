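; BP_GraphNode is a territory graph node actor that visualizes its links to neighboring nodes by color.
; AddColorToNeighbors tints its own cube teal and colors each valid entry in Connections by direction, casting the array index to a node direction and looking it up in ColorsPerDirection.
; RemoveColorFromNeighbors resets itself and its neighbors to white.
; All coloring goes through ColorSelf, which sets the Color material parameter on the cube.
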(event Custom|RemoveColorFromNeighbors
  (Class|GraphNode|ColorSelf "(R=1.000000,G=1.000000,B=1.000000,A=1.000000)")
  (Class|GraphNode|ColorNeighbors false))

(event Custom|AddColorToNeighbors
  (Class|GraphNode|ColorSelf "(R=0.066667,G=0.301961,B=0.333333,A=1.000000)")
  (Class|GraphNode|ColorNeighbors true))

(event EventBeginPlay)

(event Collision|EventActorBeginOverlap
  (params (OtherActor :type Actor%20Object%20Reference)))

(event EventTick
  (params (DeltaSeconds :type Float%20%28single-precision%29)))

(event EventColorSelf
  (params (NewColor :type Linear%20Color%20Structure))
  (Rendering|Material|SetVectorParameterValueonMaterials (Variables|Default|GetCube) "Color" (Math|Conversions|ToVector(LinearColor) NewColor)))

(event EventColorNeighbors
  (params (AddColor :type Boolean))
  (if AddColor
    (for (_array_element _array_index) (Variables|Default|GetConnections)
      (Utilities|IsValid _array_element
        (:Is%20Valid
          (Class|GraphNode|ColorSelf _array_element (.Value (Utilities|Map|Find (Variables|Default|GetColorsPerDirection) (Utilities|Enum|ByteToEnumNodeDirection (Math|Conversions|ToByte(Integer) _array_index))))))))
    (else
      (for _array_element_2 (Variables|Default|GetConnections)
        (Utilities|IsValid _array_element_2
          (:Is%20Valid
            (Class|GraphNode|ColorSelf _array_element_2 "(R=1.000000,G=1.000000,B=1.000000,A=1.000000)")))))))

(fn ConstructionScript)