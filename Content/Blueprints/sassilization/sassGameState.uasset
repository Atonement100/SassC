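; Game state for Sassilization that times the pre-game warm-up and switches PreGameActive off on Tick once it expires.
; The PreGameActive RepNotify then creates the local player's HUD and recolors every SassGamePlayer from its PlayerState color, also routing each through a server color event.
; GameBody and GameEnd are rudimentary win-condition stubs not called here, and several debug chains are disconnected.
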(event Custom|Color_Player_server
  (params (Color :type Linear%20Color%20Structure) (PlayerCharacter :type Sass%20Game%20Player%20Object%20Reference))
  (Default|ChangeColorHandler PlayerCharacter Color))

(event Custom|ColorPlayers
  (params (sassPlayer :type Sass%20Game%20Player%20Object%20Reference)))

(event EventBeginPlay)

(event EventTick
  (params (DeltaSeconds :type Float%20%28single-precision%29))
  (if (Variables|Default|GetpreGameActive)
    (Variables|Default|SettimeKeeper (+ DeltaSeconds (Variables|Default|GettimeKeeper)))
    (if (> (Variables|Default|GettimeKeeper) (Variables|Default|GetWarmUpTime))
      (Variables|Default|SetpreGameActive false))))

(fn ConstructionScript)

(fn GameBody
  (if (>= (Variables|Default|GettimeKeeper) 1e+02)
    (Variables|Default|SetwinnerDeclared true)))

(fn GameEnd
  (Development|PrintString "Player has won"))

(fn OnRepPreGameActive
  (if (not (Variables|Default|GetpreGameActive))
    (bind _assass_game_player (Utilities|Casting|CastTosassGamePlayer (Game|GetPlayerCharacter 0)))
    (Class|SassPlayer|CreateGameHUD _assass_game_player)
    (bind _returnvalue (Class|SassPlayer|GetGameWidget _assass_game_player))
    (bind _assassilization_hud_bp (Utilities|Casting|CastTosassilizationHUD_BP _returnvalue))
    (Variables|/Game/Blueprints/sassilization/sassGamePlayer.sassGamePlayer_C|SetsassHudWidget _assass_game_player _assassilization_hud_bp)
    (bind _outactors (Actor|GetAllActorsOfClass "/Game/Blueprints/sassilization/sassGamePlayer.sassGamePlayer_C"))
    (for _array_element _outactors
      (bind _assass_player_state (Utilities|Casting|CastTosassPlayerState (Variables|/Script/Engine.Pawn|GetPlayerState _array_element)))
      (Default|ChangeColor _array_element (Variables|/Script/SassC.sassPlayerState|GetPlayerColor _assass_player_state))
      (CallFunction|ColorPlayerServer (Variables|/Script/SassC.sassPlayerState|GetPlayerColor _assass_player_state) _array_element))
    (Development|PrintString (Utilities|String|ToString(Integer) (Utilities|Array|Length _outactors)) true true "(R=0.000000,G=0.660000,B=1.000000,A=1.000000)" 1e+01)))