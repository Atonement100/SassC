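; Player controller for Sassilization that handles the unit spawn menu and building spawn requests.
; It stores the Sassilization HUD widget handed to it, and the unit menu event toggles that widget's spawn menu along with cursor visibility and input mode.
; The G key requests a building spawn, while V only prints a debug message on press and release.
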(event EventUnitMenuPressed
  (Utilities|IsValid (Variables|Default|GetSassHudWidget)
    (:Is%20Valid
      (if (Variables|Default|GetbIsUnitMenuOpen)
        (Variables|Default|SetbIsUnitMenuOpen false)
        (Default|HideSpawnMenu (Variables|Default|GetSassHudWidget))
        (Variables|Default|SetbShowMouseCursor false)
        (Input|SetInputModeGameOnly self false)
        (else
          (Variables|Default|SetbIsUnitMenuOpen true)
          (Default|ShowSpawnMenu (Variables|Default|GetSassHudWidget))
          (Variables|Default|SetbShowMouseCursor true)
          (Input|SetInputModeGameandUI self 0 "DoNotLock" true false))))))

(event EventStoreGameWidget
  (params (GameWidget :type User%20Widget%20Object%20Reference))
  (Utilities|IsValid GameWidget
    (:Is%20Valid
      (bind _aswbp_sassilization_hud (Utilities|Casting|CastToWBP_SassilizationHUD GameWidget))
      (Variables|Default|SetSassHudWidget _aswbp_sassilization_hud))
    (:Is%20Not%20Valid
      (Utilities|String|LogString "Game Widget offered was not valid"))))

(event EventBeginPlay)

(event EventTick
  (params (DeltaSeconds :type Float%20%28single-precision%29)))

(event Input|KeyboardEvents|G
  (params (Key :type Key%20Structure :default "None"))
  (:Pressed
    (Class|SassPlayerController|RequestBuildingSpawn)))

(event Input|KeyboardEvents|V
  (params (Key :type Key%20Structure :default "None"))
  (:Pressed
    (Development|PrintString "intercepted VVV" :!label _label))
  (:Released
    (goto _label)))

(fn ConstructionScript)