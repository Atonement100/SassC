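; Game mode for Sassilization that sets up joining players and handles building and unit placement on the server.
; PostLogin gives each PlayerState a random color; GameBody sets a looping resource-distribution timer, while other phase functions are empty.
; Spawn requests must pass surface-normal, box-trace overlap and midpoint height checks.
; Spawned actors get owner and team color; cities also create an area of influence.
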(event Custom|RequestSetOwner
  (params (Target :type Actor%20Object%20Reference%20%28by%20ref%29) (Owner :type Actor%20Object%20Reference%20%28by%20ref%29)))

(event Custom|PlayerWantsToSpawnBldg
  (params (PlayerController :type Player%20Controller%20Object%20Reference) (ActorToSpawn :type Actor%20Class%20Reference) (HitResult :type Hit%20Result%20Structure) (currentHalfHeight :type Vector) (midpointsToCheck :type Array%20of%20Vectors))
  (bind (_bblockinghit _binitialoverlap _time _location _impactpoint _normal) (Collision|BreakHitResult HitResult))
  (if (>= (.Z (Math|Vector|BreakVector _normal)) 0.99)
    (bind _returnvalue (Class|KismetSystemLibrary|BoxTraceSingleforObjects (+ _location "0, 0,11.000000") (+ _location "0, 0,50.000000") "50.000000,50.000000,10.000000" "0, 0,0.000000" (Utilities|Array|MakeArray "ObjectTypeQuery1" "ObjectTypeQuery2") true 0 "ForOneFrame" true))
    (Variables|Default|SetisBadSpawn _returnvalue)
    (else
      (Variables|Default|SetisBadSpawn true)))
  (if (Variables|Default|GetisBadSpawn)
    (Development|PrintString "bad spawn!" :!label _label)
    (else
      (bind _isbadspawn (CallFunction|CheckCornersServer midpointsToCheck _location))
      (bind _output_get (Variables|Default|SetisBadSpawn _isbadspawn))
      (if _output_get
        (goto _label)
        (else
          (bind _returnvalue_2 (Game|SpawnActorfromClass ActorToSpawn (Math|Conversions|ToTransform(Vector) (+ _location currentHalfHeight)) "AlwaysSpawn" PlayerController 0))
          (bind _assass_player_state_bp (Utilities|Casting|CastTosassPlayerState_BP (Variables|/Script/Engine.Controller|GetPlayerState PlayerController)))
          (Utilities|Array|Add (Variables|/Game/Blueprints/sassilization/sassPlayerState_BP.sassPlayerState_BP_C|GetControlledBuildings _assass_player_state_bp) _returnvalue_2)
          (bind _asbuilding_base (Utilities|Casting|CastToBuildingBase _returnvalue_2)
            (:then
              (bind _output_get_2 (Variables|/Game/Blueprints/sassilization/BuildingBPs/BuildingBase.BuildingBase_C|SetOwningPlayerState _asbuilding_base _assass_player_state_bp))
              (Default|UpdateMaterial _asbuilding_base (Variables|/Game/Blueprints/sassilization/sassPlayerState_BP.sassPlayerState_BP_C|GetcolorOfPlayer _output_get_2) _asbuilding_base)
              (bind _ascity (Utilities|Casting|CastToCity _asbuilding_base))
              (Default|CreateAreaOfInfluence _ascity))
            (:CastFailed
              (bind _asunit_base (Utilities|Casting|CastTounitBase _returnvalue_2))
              (Variables|/Game/Blueprints/sassilization/UnitBPs/unitBase.unitBase_C|SetOwningPlayerState _asunit_base _assass_player_state_bp)
              (Default|UpdateMaterials _asunit_base (Variables|/Game/Blueprints/sassilization/sassPlayerState_BP.sassPlayerState_BP_C|GetcolorOfPlayer _assass_player_state_bp)))))))))

(event Custom|PostLoginActivities
  (params (PlayerController :type Player%20Controller%20Object%20Reference))
  ;[1 1 1] may need to move this logic elsewhere. perhaps to gamestate and handle this in pregame time rather than on connect.
  (bind _assass_player_state_bp (Utilities|Casting|CastTosassPlayerState_BP (Variables|/Script/Engine.Controller|GetPlayerState PlayerController)))
  (Variables|/Game/Blueprints/sassilization/sassPlayerState_BP.sassPlayerState_BP_C|SetcolorOfPlayer _assass_player_state_bp (CallFunction|ChoosePlayerColor))
  (Development|PrintString (Utilities|String|Append (Variables|/Script/Engine.PlayerState|GetPlayerName _assass_player_state_bp) " login success, color set")))

(event EventBeginPlay)

(event EventTick
  (params (DeltaSeconds :type Float%20%28single-precision%29)))

(event EventPostLogin
  (params (NewPlayer :type Player%20Controller%20Object%20Reference))
  (CallFunction|PostLoginActivities NewPlayer))

(fn ConstructionScript)

(fn Pregame)

(fn GameBody
  (Development|PrintString "The game has begun.")
  (Utilities|Time|SetTimerbyFunctionName "/Game/Blueprints/sassilization/sassPlayerState_BP.sassPlayerState_BP_C" "distributeResourcesPS" 1e+01 true))

(fn GameEnd)

(fn ChoosePlayerColor
  (return (Math|Color|MakeColor (Math|Random|RandomFloatinRange 0.0 1.0) (Math|Random|RandomFloatinRange 0.0 1.0) (Math|Random|RandomFloatinRange 0.0 1.0))))

(fn FindPlayerStart
  (params (Player :type Controller%20Object%20Reference) (IncomingName :type String))
  (if (== (Utilities|Array|Length (Variables|Default|GetplayerSpawns)) 0)
    (bind _outactors (Actor|GetAllActorsOfClass "/Script/Engine.PlayerStart"))
    (Variables|Default|SetplayerSpawns _outactors))
  (if (== (Utilities|Array|Length (Variables|Default|GetplayerSpawns)) 0)
    _
    (else
      (while (not (LocalVariables|GetPlayerStartFound))
        (Utilities|FlowControl|Sequence
          (:then_0
            (LocalVariables|SetPlayerStartFound true))
          (:then_1
            (Utilities|Array|RemoveItem (Variables|Default|GetplayerSpawns) (Utilities|Array|Get(acopy) (Variables|Default|GetplayerSpawns) (Math|Random|RandomIntegerinRange 0 (- (Utilities|Array|Length (Variables|Default|GetplayerSpawns)) 1)))))
          (:then_2
            (return (Utilities|Array|Get(acopy) (Variables|Default|GetplayerSpawns) (Math|Random|RandomIntegerinRange 0 (- (Utilities|Array|Length (Variables|Default|GetplayerSpawns)) 1)))))))))
  (return (LocalVariables|GetNULL_PLAYER_START)))

(fn CheckCornersServer
  (params (sideMidpoints :type Array%20of%20Vectors) (Center :type Vector))
  (bind _traceheightarray (Variables|Default|GettraceHeightArray))
  (Utilities|Array|Clear (Variables|Default|GettraceHeightArray))
  (for _array_element sideMidpoints
    (bind (_outhit _returnvalue) (Collision|LineTraceForObjects (+ _array_element Center) (- (+ _array_element Center) "0, 0,35.000000") (Utilities|Array|MakeArray "ObjectTypeQuery1") true 0 "ForOneFrame"))
    (if _returnvalue
      (Utilities|Array|Add (Variables|Default|GettraceHeightArray) (.Z (Math|Vector|BreakVector (.Location (Collision|BreakHitResult _outhit)))))
      (else
        (Development|PrintString "BAD LINE TRACE SERVER" true true "(R=1.000000,G=0.240534,B=0.000000,A=1.000000)")
        (return true))))
  (for _array_element_2 _traceheightarray
    (if (not (Math|Float|NearlyEqual(Float) _array_element_2 (Utilities|Array|Get(acopy) _traceheightarray) 6.0))
      (Development|PrintString "FLOAT NOT EQUAL SERVER" true true "(R=1.000000,G=0.329981,B=0.000000,A=1.000000)")
      (return true)))
  (return false))