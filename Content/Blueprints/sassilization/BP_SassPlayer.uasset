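; Player pawn for Sassilization that carries debug hotkeys for player state, node graph inspection and a cursor decal test.
; Keys print the player's color, controlled buildings and selected units from BP_SassPlayerState.
; A toggled per-tick trace highlights the neighbors of the hit BP_GraphNode, and another key colors the node nearest a traced point via BP_NodeManager.
; The construction script creates a dynamic mesh material with a PlayerColor parameter, initially black.
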(event EventTick
  (params (DeltaSeconds :type Float%20%28single-precision%29))
  (bind (_start _end) (Utilities|GetRaycastVectors))
  (if (Variables|Default|GetShouldRaycast)
    (bind (_outhit _returnvalue) (Collision|LineTraceByChannel _start _end "TraceTypeQuery8" true 0 "ForOneFrame"))
    (if _returnvalue
      (bind _asbp_graph_node (Utilities|Casting|CastToBP_GraphNode (.HitActor (Collision|BreakHitResult _outhit))))
      (Default|RemoveColorfromNeighbors (Variables|Default|GetLastNodeSeen))
      (bind _output_get (Variables|Default|SetLastNodeSeen _asbp_graph_node))
      (Default|ColorNeighbors _output_get true))))

(event Input|KeyboardEvents|T
  (params (Key :type Key%20Structure :default "None"))
  (:Pressed
    (bind _output_get (Variables|Default|SetShouldRaycast (not (Variables|Default|GetShouldRaycast))))
    (if (not _output_get)
      (Default|RemoveColorfromNeighbors (Variables|Default|GetLastNodeSeen)))))

(event Input|KeyboardEvents|V
  (params (Key :type Key%20Structure :default "None"))
  (bind (_start _end) (Utilities|GetRaycastVectors))
  (:Pressed
    (bind (_outhit _returnvalue) (Collision|LineTraceByChannel _start _end "TraceTypeQuery1" true 0 "ForDuration"))
    (if _returnvalue
      (bind _returnvalue_2 (Actor|GetActorOfClass "/Game/Blueprints/sassilization/Territory/BP_NodeManager.BP_NodeManager_C"))
      (bind (_graphnode _foundnode) (Default|FindNearestNodeBP _returnvalue_2 (.Location (Collision|BreakHitResult _outhit)) 16.0))
      (if _foundnode
        (Default|ColorSelf _graphnode "(R=0.000000,G=1.000000,B=0.262745,A=1.000000)"))))
  (:Released
    (Default|ColorSelf _graphnode "(R=1.000000,G=1.000000,B=1.000000,A=1.000000)")))

(event Input|KeyboardEvents|X
  (params (Key :type Key%20Structure :default "None"))
  ;[1 1 1] implement sprays?
  (:Pressed
    (Rendering|Decal|SpawnDecalatLocation "/Game/Blueprints/sassilization/BuildingModels/tower/archertower_material.archertower_material" "50.000000,50.000000,50.000000" (.Location (Collision|BreakHitResult (.HitResult (Game|Player|GetHitResultUnderCursorbyChannel (Game|GetPlayerController 0) "TraceTypeQuery1" true)))) "-90.000000,0.000000,0.000000" 0.0)))

(event Input|KeyboardEvents|H
  (params (Key :type Key%20Structure :default "None"))
  ;[1 1 1] Temp Function to show colors on request via text...
  (:Pressed
    (bind _asbp_sass_player_state (Utilities|Casting|CastToBP_SassPlayerState (Variables|Default|GetPlayerState)))
    (Development|PrintString (Utilities|String|ToString(Integer) (Variables|/Script/SassC.SassPlayerState|GetPlayerColor _asbp_sass_player_state)) true true (Variables|/Script/SassC.SassPlayerState|GetPlayerColor _asbp_sass_player_state))))

(event Input|KeyboardEvents|C
  (params (Key :type Key%20Structure :default "None"))
  (:Pressed
    (Development|PrintString "SELECTED UNITS:" true true "(R=0.000000,G=0.660000,B=1.000000,A=1.000000)" 1e+01)
    (for _array_element (Variables|/Script/SassC.SassPlayerState|GetSelectedUnits (.AsBP%20Sass%20Player%20State (Utilities|Casting|CastToBP_SassPlayerState (Variables|Default|GetPlayerState))))
      (Development|PrintString (Utilities|String|ToString(Object) _array_element) true true "(R=0.000000,G=0.660000,B=1.000000,A=1.000000)" 1e+01))
    (Development|PrintString "donello")))

(event Input|KeyboardEvents|G
  (params (Key :type Key%20Structure :default "None"))
  (:Pressed
    (Development|PrintString "start")
    (for _array_element (Variables|/Script/SassC.SassPlayerState|GetControlledBuildings (.AsBP%20Sass%20Player%20State (Utilities|Casting|CastToBP_SassPlayerState (Variables|Default|GetPlayerState))))
      (Development|PrintString (Utilities|String|ToString(Object) _array_element)))
    (Development|PrintString "done")))

(fn ConstructionScript
  (bind _returnvalue (Rendering|Material|CreateDynamicMaterialInstance (Variables|Character|GetMesh) 0 (Rendering|Material|GetMaterial (Variables|Character|GetMesh) 0) "None" :!class /Script/Engine.PrimitiveComponent))
  (Rendering|Material|SetVectorParameterValue _returnvalue "PlayerColor" "(R=0.000000,G=0.000000,B=0.000000,A=1.000000)" :!class /Script/Engine.MaterialInstanceDynamic)
  (bind _output_get (Variables|Default|SetDynamicPlayerMaterial _returnvalue))
  (Rendering|Material|SetMaterial 0 _output_get))