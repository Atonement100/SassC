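; Game mode Blueprint for Sassilization that handles match start-up and player spawn selection.
; GameBody announces the game start and sets a looping timer that calls distributeResourcesPS on the player state for periodic resource distribution.
; FindPlayerStart caches all PlayerStart actors, removes a random entry and returns a separately randomized one, guarded by a PlayerStartFound flag that is never reset here.
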(fn ConstructionScript)

(fn GameBody
  (Development|PrintString "The game has begun.")
  (Utilities|Time|SetTimerbyFunctionName "/Game/Blueprints/sassilization/sassPlayerState_BP.sassPlayerState_BP_C" "distributeResourcesPS" 1e+01 true))

(fn FindPlayerStart
  (params (Player :type Controller%20Object%20Reference) (IncomingName :type String))
  (if (== (Utilities|Array|Length (Variables|Default|GetplayerSpawns_1)) 0)
    (bind _outactors (Actor|GetAllActorsOfClass "/Script/Engine.PlayerStart"))
    (Variables|Default|SetplayerSpawns_1 _outactors))
  (if (== (Utilities|Array|Length (Variables|Default|GetplayerSpawns_1)) 0)
    _
    (else
      (while (not (LocalVariables|GetPlayerStartFound))
        (Utilities|FlowControl|Sequence
          (:then_0
            (LocalVariables|SetPlayerStartFound true))
          (:then_1
            (Utilities|Array|RemoveItem (Variables|Default|GetplayerSpawns_1) (Utilities|Array|Get(acopy) (Variables|Default|GetplayerSpawns_1) (Math|Random|RandomIntegerinRange 0 (- (Utilities|Array|Length (Variables|Default|GetplayerSpawns_1)) 1)))))
          (:then_2
            (return (Utilities|Array|Get(acopy) (Variables|Default|GetplayerSpawns_1) (Math|Random|RandomIntegerinRange 0 (- (Utilities|Array|Length (Variables|Default|GetplayerSpawns_1)) 1)))))))))
  (return (LocalVariables|GetNULL_PLAYER_START)))