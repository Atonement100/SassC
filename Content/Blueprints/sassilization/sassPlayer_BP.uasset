(event EventOpenUnitMenu
  ;[1 1 1] (BlueprintNative) Unit Menus
  (Widget|SetVisibility (Variables|/Game/Blueprints/sassilization/sassilizationHUD_BP.sassilizationHUD_BP_C|GetUnitAndBldgBackground (Variables|Default|GetsassHudWidget)) "HitTestInvisible")
  (Widget|SetVisibility (Variables|/Game/Blueprints/sassilization/sassilizationHUD_BP.sassilizationHUD_BP_C|GetUnitBldgButtonSwitcher (Variables|Default|GetsassHudWidget)) "SelfHitTestInvisible")
  (Widget|SetVisibility (Variables|/Game/Blueprints/sassilization/sassilizationHUD_BP.sassilizationHUD_BP_C|GetUnitToBldgButtonOverlay (Variables|Default|GetsassHudWidget)) "SelfHitTestInvisible"))

(event EventCloseUnitMenu
  ;[1 1 1] (BlueprintNative) Unit Menus
  (Widget|SetVisibility (Variables|/Game/Blueprints/sassilization/sassilizationHUD_BP.sassilizationHUD_BP_C|GetUnitAndBldgBackground (Variables|Default|GetsassHudWidget)) "Collapsed")
  (Widget|SetVisibility (Variables|/Game/Blueprints/sassilization/sassilizationHUD_BP.sassilizationHUD_BP_C|GetUnitBldgButtonSwitcher (Variables|Default|GetsassHudWidget)) "Collapsed")
  (Widget|SetVisibility (Variables|/Game/Blueprints/sassilization/sassilizationHUD_BP.sassilizationHUD_BP_C|GetUnitToBldgButtonOverlay (Variables|Default|GetsassHudWidget)) "Collapsed"))

(event EventSetSassHUDRef
  ;[1 1 1] (BlueprintNative) Best interface to deal with widgets from code
  (bind _assassilization_hud_bp (Utilities|Casting|CastTosassilizationHUD_BP (Variables|Default|GetGameWidget)))
  (Variables|Default|SetsassHudWidget _assassilization_hud_bp))

(event Input|ActionEvents|InputActionRightClick
  (params (Key :type Key%20Structure :default "AnyKey"))
  ;[1 1 1] right click
)

(event Input|KeyboardEvents|X
  (params (Key :type Key%20Structure :default "AnyKey"))
  ;[1 1 1] implement sprays?
  (:Pressed
    (Rendering|Decal|SpawnDecalatLocation "/Game/Blueprints/sassilization/ownerZone.ownerZone" "50.000000,50.000000,50.000000" (.Location (Collision|BreakHitResult (.HitResult (Game|Player|GetHitResultUnderCursorbyChannel (Game|GetPlayerController 0) "TraceTypeQuery1" true)))) "-90.000000,0.000000,0.000000" 0.0)
    (Development|PrintString "complete")))

(event Input|KeyboardEvents|H
  (params (Key :type Key%20Structure :default "AnyKey"))
  ;[1 1 1] Temp Function to show colors on request via text...
  (:Pressed
    (bind _assass_player_state_bp (Utilities|Casting|CastTosassPlayerState_BP (Variables|Default|GetPlayerState)))
    (Development|PrintString (Utilities|String|ToString(Integer) (Variables|/Script/SassC.sassPlayerState|GetPlayerColor _assass_player_state_bp)) true true (Variables|/Script/SassC.sassPlayerState|GetPlayerColor _assass_player_state_bp))))

(event Input|KeyboardEvents|C
  (params (Key :type Key%20Structure :default "AnyKey"))
  (:Pressed
    (Development|PrintString "SELECTED UNITS:" true true "(R=0.000000,G=0.660000,B=1.000000,A=1.000000)" 1e+01)
    (for _array_element (Variables|/Script/SassC.sassPlayerState|GetSelectedUnits (.AsSass%20Player%20State%20BP (Utilities|Casting|CastTosassPlayerState_BP (Variables|Default|GetPlayerState))))
      (Development|PrintString (Utilities|String|ToString(Object) _array_element) true true "(R=0.000000,G=0.660000,B=1.000000,A=1.000000)" 1e+01))
    (Development|PrintString "donello")))

(event Input|KeyboardEvents|G
  (params (Key :type Key%20Structure :default "AnyKey"))
  (:Pressed
    (Development|PrintString "start")
    (for _array_element (Variables|/Script/SassC.sassPlayerState|GetControlledBuildings (.AsSass%20Player%20State%20BP (Utilities|Casting|CastTosassPlayerState_BP (Variables|Default|GetPlayerState))))
      (Development|PrintString (Utilities|String|ToString(Object) _array_element)))
    (Development|PrintString "done")))

(fn ConstructionScript
  (bind _returnvalue (Rendering|Material|CreateDynamicMaterialInstance (Variables|Character|GetMesh) 0 (Rendering|Material|GetMaterial (Variables|Character|GetMesh) 0) :!class /Script/Engine.PrimitiveComponent))
  (Rendering|Material|SetVectorParameterValue _returnvalue "PlayerColor" "(R=0.000000,G=0.000000,B=0.000000,A=1.000000)" :!class /Script/Engine.MaterialInstanceDynamic)
  (bind _output_get (Variables|Default|SetDynamicPlayerMaterial _returnvalue))
  (Rendering|Material|SetMaterial 0 _output_get))