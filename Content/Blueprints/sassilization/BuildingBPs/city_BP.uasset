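; City building Blueprint for Sassilization whose only working logic is SortBoundaries, which orders boundary points by angle around a center point.
; It takes each point's Atan2 angle in degrees and insertion-sorts it into DegreeArray, mirroring each insert in SortedBoundaries, which it returns.
; The event graph and construction script are empty, and a leftover comparison branch never runs.
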(event EventBeginPlay)

(event Collision|EventActorBeginOverlap
  (params (OtherActor :type Actor%20Object%20Reference)))

(event EventTick
  (params (DeltaSeconds :type Float%20%28single-precision%29)))

(fn ConstructionScript)

(fn SortBoundaries
  (params (boundaries :type Array%20of%20Vectors) (center :type Vector))
  (bind (_x _y) (Math|Vector|BreakVector center))
  (bind _degreearray (LocalVariables|GetdegreeArray))
  (bind _degreearray_2 (LocalVariables|GetdegreeArray))
  (LocalVariables|SetcenterX _x)
  (LocalVariables|SetcenterY _y)
  (Utilities|Array|Clear _degreearray)
  (for _array_element boundaries
    (if (or (== (Utilities|Array|Length _degreearray) 0) (> (Class|KismetMathLibrary|DegAtan2 (- (.Y (Math|Vector|BreakVector _array_element)) (LocalVariables|GetcenterY)) (- (.X (Math|Vector|BreakVector _array_element)) (LocalVariables|GetcenterX))) (Utilities|Array|Get(acopy) _degreearray (Utilities|Array|LastIndex _degreearray))))
      (Utilities|Array|Add (LocalVariables|GetdegreeArray) (Class|KismetMathLibrary|DegAtan2 (- (.Y (Math|Vector|BreakVector _array_element)) (LocalVariables|GetcenterY)) (- (.X (Math|Vector|BreakVector _array_element)) (LocalVariables|GetcenterX))))
      (Utilities|Array|Add (LocalVariables|GetsortedBoundaries) _array_element)
      (else
        (bind _index (Utilities|FlowControl|ForLoopwithBreak 0 (- (Utilities|Array|Length _degreearray_2) 1) :!label _label)
          (:LoopBody
            (if (< (Class|KismetMathLibrary|DegAtan2 (- (.Y (Math|Vector|BreakVector _array_element)) (LocalVariables|GetcenterY)) (- (.X (Math|Vector|BreakVector _array_element)) (LocalVariables|GetcenterX))) (Utilities|Array|Get(acopy) _degreearray_2 _index))
              (Utilities|Array|Insert (LocalVariables|GetdegreeArray) (Class|KismetMathLibrary|DegAtan2 (- (.Y (Math|Vector|BreakVector _array_element)) (LocalVariables|GetcenterY)) (- (.X (Math|Vector|BreakVector _array_element)) (LocalVariables|GetcenterX))) _index)
              (Utilities|Array|Insert (LocalVariables|GetsortedBoundaries) _array_element _index)
              (goto _label Break)))))))
  (return (LocalVariables|GetsortedBoundaries)))